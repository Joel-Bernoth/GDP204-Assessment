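; Ordered-button puzzle that spawns the cat Gerald at the puzzle actor's location when solved.
; InteractedWithPuzzlePiece sets a flag per piece ID only if the required earlier flags are set; otherwise ResetPuzzle clears all six.
; The sequence follows ID order except the last two, which are swapped.
; Tick polls the flags and, through a DoOnce, spawns CatBase_Char with the "gerald" row from the Catopedia table.
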(event Custom|Interacted%20With%20Puzzle%20Piece
  (params (ID :type Integer))
  (switch int ID
    (:0
      (Variables|Default|SetButton1 true)
      (Development|PrintString "Hello"))
    (:1
      (if (Variables|Default|GetButton1)
        (Variables|Default|SetButton2 true)
        (else
          (CallFunction|ResetPuzzle))))
    (:2
      (if (and (Variables|Default|GetButton1) (Variables|Default|GetButton2))
        (Variables|Default|SetButton3 true)
        (else
          (CallFunction|ResetPuzzle))))
    (:3
      (if (Math|Boolean|ANDBoolean (Variables|Default|GetButton1) (Variables|Default|GetButton2) (Variables|Default|GetButton3))
        (Variables|Default|SetButton4 true)
        (else
          (CallFunction|ResetPuzzle))))
    (:4
      (if (Math|Boolean|ANDBoolean (Variables|Default|GetButton1) (Variables|Default|GetButton2) (Variables|Default|GetButton3) (Variables|Default|GetButton4) (Variables|Default|GetButton6))
        (Variables|Default|SetButton5 true)
        (else
          (CallFunction|ResetPuzzle))))
    (:5
      (if (Math|Boolean|ANDBoolean (Variables|Default|GetButton1) (Variables|Default|GetButton2) (Variables|Default|GetButton3) (Variables|Default|GetButton4))
        (Variables|Default|SetButton6 true)
        (else
          (CallFunction|ResetPuzzle))))))

(event EventTick
  (params (DeltaSeconds :type Float%20%28single-precision%29))
  (if (Math|Boolean|ANDBoolean (Variables|Default|GetButton1) (Variables|Default|GetButton2) (Variables|Default|GetButton3) (Variables|Default|GetButton4) (Variables|Default|GetButton5) (Variables|Default|GetButton6))
    (Utilities|FlowControl|DoOnce false
      (:Completed
        (Game|SpawnActorfromClass "/Game/Cats/CatBase_Char.CatBase_Char_C" (Math|Transform|MakeTransform (Transformation|GetActorLocation) "0, 0, 0" "1.000000,1.000000,1.000000") "Undefined" 0 (Utilities|Struct|MakeDataTableRowHandle "/Game/Cats/Catopedia.Catopedia" "gerald") 0)))))

(fn ConstructionScript
  (|CallParentFunction))

(fn ResetPuzzle
  (Variables|Default|SetButton1 false)
  (Variables|Default|SetButton2 false)
  (Variables|Default|SetButton3 false)
  (Variables|Default|SetButton4 false)
  (Variables|Default|SetButton5 false)
  (Variables|Default|SetButton6 false)
  (return))
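; BP_Background is one map tile that links to up to four neighbors for screen-by-screen travel and sets its picture through a dynamic material.
; Edge colliders block without a neighbor; otherwise overlap blends the camera to that tile, teleports NekoRyoshi to its opposite spawn and updates HUD coordinates.
; When AssetsEnabled, BeginPlay scatters trees, bushes and rocks using random line traces that hit a background, with small rocks ignoring collision.
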(event OnComponentBeginOverlap(Collider_BOTTOM)
  (params (OverlappedComponent :type Primitive%20Component%20Object%20Reference) (OtherActor :type Actor%20Object%20Reference) (OtherComp :type Primitive%20Component%20Object%20Reference) (OtherBodyIndex :type Integer) (bFromSweep :type Boolean) (SweepResult :type Hit%20Result%20Structure%20%28by%20ref%29))
  (bind _asneko_ryoshi (Utilities|Casting|CastToNekoRyoshi OtherActor))
  (bind _down (Variables|Default|GetDown)
    (:then
      (Game|Player|SetViewTargetwithBlend (Game|GetPlayerController 0) _down 0.0 "VTBlend_Linear" 0.0 false)
      (Transformation|Teleport _asneko_ryoshi (Transformation|GetWorldLocation (Variables|BP_Background_C|GetTop_Spawn _down)) (Transformation|GetActorRotation _asneko_ryoshi))
      (Variables|/Game/Player/HUD/HUD.HUD_C|SetXCoord_V (Variables|/Game/Player/NekoRyoshi.NekoRyoshi_C|GetPlayerHud _asneko_ryoshi) (Variables|BP_Background_C|GetXCoordinate _down))
      (Variables|/Game/Player/HUD/HUD.HUD_C|SetYCoord_V (Variables|/Game/Player/NekoRyoshi.NekoRyoshi_C|GetPlayerHud _asneko_ryoshi) (Variables|BP_Background_C|GetYCoordinate _down)))
    (:else)))

(event OnComponentBeginOverlap(Collider_TOP)
  (params (OverlappedComponent :type Primitive%20Component%20Object%20Reference) (OtherActor :type Actor%20Object%20Reference) (OtherComp :type Primitive%20Component%20Object%20Reference) (OtherBodyIndex :type Integer) (bFromSweep :type Boolean) (SweepResult :type Hit%20Result%20Structure%20%28by%20ref%29))
  (bind _asneko_ryoshi (Utilities|Casting|CastToNekoRyoshi OtherActor))
  (bind _up (Variables|Default|GetUp)
    (:then
      (Game|Player|SetViewTargetwithBlend (Game|GetPlayerController 0) _up 0.0 "VTBlend_Linear" 0.0 false)
      (Transformation|Teleport _asneko_ryoshi (Transformation|GetWorldLocation (Variables|BP_Background_C|GetBottom_Spawn _up)) (Transformation|GetActorRotation _asneko_ryoshi))
      (Variables|/Game/Player/HUD/HUD.HUD_C|SetXCoord_V (Variables|/Game/Player/NekoRyoshi.NekoRyoshi_C|GetPlayerHud _asneko_ryoshi) (Variables|BP_Background_C|GetXCoordinate _up))
      (Variables|/Game/Player/HUD/HUD.HUD_C|SetYCoord_V (Variables|/Game/Player/NekoRyoshi.NekoRyoshi_C|GetPlayerHud _asneko_ryoshi) (Variables|BP_Background_C|GetYCoordinate _up)))
    (:else)))

(event OnComponentBeginOverlap(Collider_RIGHT)
  (params (OverlappedComponent :type Primitive%20Component%20Object%20Reference) (OtherActor :type Actor%20Object%20Reference) (OtherComp :type Primitive%20Component%20Object%20Reference) (OtherBodyIndex :type Integer) (bFromSweep :type Boolean) (SweepResult :type Hit%20Result%20Structure%20%28by%20ref%29))
  (bind _asneko_ryoshi (Utilities|Casting|CastToNekoRyoshi OtherActor))
  (bind _right (Variables|Default|GetRight)
    (:then
      (Game|Player|SetViewTargetwithBlend (Game|GetPlayerController 0) _right 0.0 "VTBlend_Linear" 0.0 false)
      (Transformation|Teleport _asneko_ryoshi (Transformation|GetWorldLocation (Variables|BP_Background_C|GetLeft_Spawn _right)) (Transformation|GetActorRotation _asneko_ryoshi))
      (Variables|/Game/Player/HUD/HUD.HUD_C|SetXCoord_V (Variables|/Game/Player/NekoRyoshi.NekoRyoshi_C|GetPlayerHud _asneko_ryoshi) (Variables|BP_Background_C|GetXCoordinate _right))
      (Variables|/Game/Player/HUD/HUD.HUD_C|SetYCoord_V (Variables|/Game/Player/NekoRyoshi.NekoRyoshi_C|GetPlayerHud _asneko_ryoshi) (Variables|BP_Background_C|GetYCoordinate _right)))
    (:else)))

(event OnComponentBeginOverlap(Collider_LEFT)
  (params (OverlappedComponent :type Primitive%20Component%20Object%20Reference) (OtherActor :type Actor%20Object%20Reference) (OtherComp :type Primitive%20Component%20Object%20Reference) (OtherBodyIndex :type Integer) (bFromSweep :type Boolean) (SweepResult :type Hit%20Result%20Structure%20%28by%20ref%29))
  (bind _asneko_ryoshi (Utilities|Casting|CastToNekoRyoshi OtherActor))
  (bind _left (Variables|Default|GetLeft)
    (:then
      (Game|Player|SetViewTargetwithBlend (Game|GetPlayerController 0) _left 0.0 "VTBlend_Linear" 0.0 false)
      (Transformation|Teleport _asneko_ryoshi (Transformation|GetWorldLocation (Variables|BP_Background_C|GetRight_Spawn _left)) (Transformation|GetActorRotation _asneko_ryoshi))
      (Variables|/Game/Player/HUD/HUD.HUD_C|SetXCoord_V (Variables|/Game/Player/NekoRyoshi.NekoRyoshi_C|GetPlayerHud _asneko_ryoshi) (Variables|BP_Background_C|GetXCoordinate _left))
      (Variables|/Game/Player/HUD/HUD.HUD_C|SetYCoord_V (Variables|/Game/Player/NekoRyoshi.NekoRyoshi_C|GetPlayerHud _asneko_ryoshi) (Variables|BP_Background_C|GetYCoordinate _left)))
    (:else)))

(event EventBeginPlay
  (bind _returnvalue (Transformation|GetActorLocation))
  (bind _xsize (Variables|Default|GetXSize))
  (bind _ysize (Variables|Default|GetYSize))
  (bind _returnvalue_2 (+ _returnvalue "0,0,9000.000000"))
  (bind _returnvalue_3 (* _ysize -1.0))
  (bind _returnvalue_4 (* _xsize -1.0))
  (bind _returnvalue_5 (Math|Random|RandomFloatinRange _returnvalue_3 _ysize))
  (bind _returnvalue_6 (Math|Random|RandomFloatinRange _returnvalue_4 _xsize))
  (bind _returnvalue_7 (+ _returnvalue_2 (Math|Vector|MakeVector _returnvalue_6 _returnvalue_5 0.0)))
  (Utilities|FlowControl|Sequence
    (:then_0
      (Utilities|CollisionCheck (Variables|Default|GetCollider_LEFT) (Variables|Default|GetLeft)))
    (:then_1
      (Utilities|CollisionCheck (Variables|Default|GetCollider_RIGHT) (Variables|Default|GetRight)))
    (:then_2
      (Utilities|CollisionCheck (Variables|Default|GetCollider_TOP) (Variables|Default|GetUp)))
    (:then_3
      (Utilities|CollisionCheck (Variables|Default|GetCollider_BOTTOM) (Variables|Default|GetDown)))
    (:then_4
      (if (Variables|Default|GetAssetsEnabled)
        (for _index (range 1 (Variables|Default|GetNumOfTrees))
          (bind _outhit (Collision|LineTraceByChannel (Math|Vector|MakeVector (.x _returnvalue_7) (.y _returnvalue_7) (.z _returnvalue_7)) (+ (+ _returnvalue "0,0,-9000.000000") (Math|Vector|MakeVector _returnvalue_6 _returnvalue_5 0.0)) "TraceTypeQuery1" false 0 "ForDuration" false))
          (Utilities|Casting|CastToBP_Background (.HitActor (Collision|BreakHitResult _outhit)))
          (switch int (Math|Random|RandomIntegerinRange 0 2)
            (:0
              (Game|SpawnActorfromClass "/Game/MAP/Trees/Trees.Trees_C" (Math|Transform|MakeTransform (+ (.ImpactPoint (Collision|BreakHitResult _outhit)) "0,0,5.000000") "0, 0, 0" "1.000000,1.000000,1.000000") "Undefined" 0 (Variables|Default|GetTree%20Sprite) 0))
            (:1
              (Game|SpawnActorfromClass "/Game/MAP/Bushes/Bushes.Bushes_C" (Math|Transform|MakeTransform (+ (.ImpactPoint (Collision|BreakHitResult _outhit)) "0,0,5.000000") "0, 0, 0" "1.000000,1.000000,1.000000") "Undefined" 0 (Variables|Default|GetBushSprite) 0))
            (:2
              (switch int (Math|Random|RandomIntegerinRange 0 2)
                (:0
                  (Game|SpawnActorfromClass "/Game/MAP/Rocks/Rocks.Rocks_C" (Math|Transform|MakeTransform (+ (.ImpactPoint (Collision|BreakHitResult _outhit)) "0,0,5.000000") "0, 0, 0" "1.000000,1.000000,1.000000") "Undefined" 0 (Variables|Default|GetLargeRockSprite) false 0))
                (:1
                  (Game|SpawnActorfromClass "/Game/MAP/Rocks/Rocks.Rocks_C" (Math|Transform|MakeTransform (+ (.ImpactPoint (Collision|BreakHitResult _outhit)) "0,0,5.000000") "0, 0, 0" "1.000000,1.000000,1.000000") "Undefined" 0 (Variables|Default|GetMediumRockSprite) false 0))
                (:2
                  (bind _returnvalue_8 (Game|SpawnActorfromClass "/Game/MAP/Rocks/Rocks.Rocks_C" (Math|Transform|MakeTransform (+ (.ImpactPoint (Collision|BreakHitResult _outhit)) "0,0,5.000000") "0, 0, 0" "1.000000,1.000000,1.000000") "Undefined" 0 (Variables|Default|GetSmallRockSprite) true 0))
                  (Collision|SetCollisionResponsetoAllChannels (Variables|/Game/MAP/Rocks/Rocks.Rocks_C|GetBox _returnvalue_8) "ECR_Ignore"))))))))))

(fn ConstructionScript
  (Utilities|FlowControl|Sequence
    (:then_0
      (bind _returnvalue (Rendering|Material|CreateDynamicMaterialInstance (Variables|Default|GetBackground) 0 "/Game/MAP/Backgrounds/M_Background.M_Background" "None" :!class /Script/Engine.PrimitiveComponent))
      (bind _output_get (Variables|Default|SetBackgroundMaterial _returnvalue))
      (Rendering|Material|SetTextureParameterValue _output_get "Picture" (Variables|Default|GetTexture)))))